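; Player character Blueprint for an RPG, handling walk/run movement, a weapon-drawn toggle and hold-to-rotate camera with a visible mouse cursor.
; Move axes drive input along the actor's forward and right vectors, scaled down unless Run is held.
; Toggling the weapon switches OrientRotationToMovement off when drawn and on when holstered.
; A Gate opened by CameraRotation lets MouseX yaw the spring arm in fixed steps beyond a dead zone.
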(event EventBeginPlay
  (Variables|/Script/Engine.PlayerController|SetbShowMouseCursor (Game|GetPlayerController 0) true))

(event Input|ActionEvents|InputActionRun
  (params (Key :type Key%20Structure))
  (:Pressed
    (Variables|Default|SetisRun true))
  (:Released
    (Variables|Default|SetisRun false)))

(event Input|ActionEvents|InputActionCameraRotation
  (params (Key :type Key%20Structure))
  (bind _springarm (Variables|Default|GetSpringArm))
  (bind _springarm_2 (Variables|Default|GetSpringArm))
  (bind _returnvalue (Class|SpringArmComponent|GetTargetRotation _springarm))
  (bind (_roll _pitch _yaw) (Math|Rotator|BreakRotator _returnvalue))
  (:Pressed
    (Utilities|FlowControl|Gate true) ; enters at Open
  )
  (:Released
    (Utilities|FlowControl|Gate true) ; enters at Close
  ))

(event Input|ActionEvents|InputActionGetWeapon
  (params (Key :type Key%20Structure))
  (bind _charactermovement (Variables|Character|GetCharacterMovement))
  (:Pressed
    (if (Variables|Default|GetWeaponOn)
      (Variables|Default|SetWeaponOn false)
      (Variables|/Script/Engine.CharacterMovementComponent|SetbOrientRotationToMovement _charactermovement true)
      (else
        (Variables|Default|SetWeaponOn true)
        (Variables|/Script/Engine.CharacterMovementComponent|SetbOrientRotationToMovement _charactermovement false)))))

(event Input|AxisEvents|InputAxisMoveRL
  (params (AxisValue :type Float%20%28single-precision%29))
  (bind _returnvalue (Transformation|GetActorRightVector))
  (if (Variables|Default|GetisRun)
    (bind _output_get (Variables|Default|SetxSpeed AxisValue))
    (Pawn|Input|AddMovementInput _returnvalue _output_get false)
    (else
      (bind _output_get_2 (Variables|Default|SetxSpeed (* AxisValue 0.6)))
      (Pawn|Input|AddMovementInput _returnvalue (* _output_get_2 1.0) false))))

(event Input|AxisEvents|InputAxisMouseX
  (params (AxisValue :type Float%20%28single-precision%29))
  (bind _springarm (Variables|Default|GetSpringArm))
  (bind _springarm_2 (Variables|Default|GetSpringArm))
  (bind _returnvalue (Class|SpringArmComponent|GetTargetRotation _springarm))
  (bind (_roll _pitch _yaw) (Math|Rotator|BreakRotator _returnvalue))
  (Utilities|FlowControl|Gate true
    (:Exit
      (if (not (== AxisValue 0.0))
        (if (> AxisValue (Variables|Default|GetMinRotationSensative))
          (Transformation|SetRelativeRotation _springarm_2 (Math|Rotator|MakeRotator _roll _pitch (+ _yaw (Variables|Default|GetRotaionSensitivityX))) false false)
          (elif (< AxisValue (* (Variables|Default|GetMinRotationSensative) -1.0))
            (Transformation|SetRelativeRotation _springarm_2 (Math|Rotator|MakeRotator _roll _pitch (- _yaw (Variables|Default|GetRotaionSensitivityX))) false false)))))))

(event Input|AxisEvents|InputAxisMoveFB
  (params (AxisValue :type Float%20%28single-precision%29))
  (bind _returnvalue (Transformation|GetActorForwardVector))
  (if (Variables|Default|GetisRun)
    (bind _output_get (Variables|Default|SetySpeed AxisValue))
    (Pawn|Input|AddMovementInput _returnvalue _output_get true)
    (else
      (bind _output_get_2 (Variables|Default|SetySpeed (* AxisValue 0.6)))
      (Pawn|Input|AddMovementInput _returnvalue _output_get_2 true))))

(fn ConstructionScript)